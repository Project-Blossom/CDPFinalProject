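; BP_Bolt is a bolt item that serves as a fixed anchor grip point, apparently for climbing.
; FindNearestGripPoint succeeds only when the search origin lies inside the GripRegion sphere, ignoring the passed search radius.
; It then returns the GripPoint location as an Anchor grip with fixed quality and angle, using the negated world position as both normals.
; The event graph and construction script are empty.
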(event EventBeginPlay)

(event Collision|EventActorBeginOverlap
  (params (OtherActor :type Actor%20Object%20Reference)))

(event EventTick
  (params (DeltaSeconds :type Float%20%28single-precision%29)))

(fn ConstructionScript)

(fn FindNearestGripPoint
  (params (SearchOrigin :type Vector%20%28by%20ref%29 :default "0, 0, 0") (SearchRadius :type Float%20%28single-precision%29))
  (bind _gripregion (Variables|Default|GetGripRegion))
  (bind _grippoint (Variables|Default|GetGripPoint))
  (bind _returnvalue (Transformation|GetWorldLocation _grippoint))
  (bind _returnvalue_2 (* _returnvalue -1.0))
  (if (<= (Math|Vector|VectorLength (- SearchOrigin (Transformation|GetWorldLocation _gripregion))) (Components|Sphere|GetScaledSphereRadius _gripregion))
    (return (Utilities|Struct|MakeGripPointInfo _returnvalue _returnvalue_2 5.0 9e+01 _returnvalue_2 true self "Anchor") true)
    (else
      (return "" false))))